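; Ratkin slave AI character that wanders around its spawn point and, if aggressive, attacks a player it perceives.
; Patrol loops through AI MoveTo to random reachable points with random pauses until an AI Perception update triggers aggro.
; Combat moves into attack range and cycles through attack montages in order, re-checking range after each.
; A looping timer checks the leash radius from spawn, resetting the target and walking it home to resume patrol.
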(event `self.ReceiveBeginPlay`
  (set `self.Startinglocation` (`self.K2_GetActorLocation`))
  (set `CharacterMovementComponent.MaxWalkSpeed` 200.0 (`self.CharacterMovement`))
  (`|AIMoveTo` self (`NavigationSystem.K2_GetRandomReachablePointInRadius` (`self.Startinglocation`) (`self.protolRadius`)) :!label _label
    (:`then`
      _)
    (:`OnSuccess`
      _))
  (if (`self.ispatroling?`)
    (`KismetSystemLibrary.Delay` (`KismetMathLibrary.RandomFloatInRange` 1.0 4.0))
    (if (`self.ispatroling?`)
      (`self.Patrol`))))

(event `Patrol`
  (goto _label))

(event `self.AIPerception.OnPerceptionUpdated`
  (params (UpdatedActors :type "Array of Actor Object Reference"))
  (if (and (not (`self.wasaggroed?`)) (`self.Aggresive?`))
    (for _array_element UpdatedActors
      (bind _asinventory_player_character (cast `/Game/InventorySystem/Blueprints/InventoryPlayerCharacter` _array_element))
      (`self.onAggropulled` _asinventory_player_character)
      (break))))

(event `PerformAttack`
  (if (not (`self.isdead?`))
    (`self.K2_SetActorRotation` (`KismetMathLibrary.FindLookAtRotation` (`self.K2_GetActorLocation` self) (`self.K2_GetActorLocation` (`self.TargetActor`))))
    (bind _output_get (set `self.CurrentAttackMontage` (`|GetArrayItem` (`self.AttackAnimations`) (`self.CurrentAnimationIndex`))))
    (`self.PlayAnimMontage` _output_get)
    (`KismetSystemLibrary.Delay` (`AnimSequenceBase.SequenceLength` _output_get))
    (set `self.CurrentAttackMontage` null)
    (set `self.CurrentAnimationIndex` (`self.getnextanimaionIndex`))
    (if (`self.inAttackrange?`)
      (`self.PerformAttack`)
      (else
        (`|AIMoveTo` self (0.0 0.0 0.0) (`self.TargetActor`) (`self.Attackrange`)
          (:`OnSuccess`
            (`self.PerformAttack`)))))))

(event `onAggropulled`
  (params (Target :type "Actor Object Reference"))
  (if (and (not (`self.wasaggroed?`)) (not (`self.isrunningback?`)))
    (set `self.ispatroling?` false)
    (set `self.wasaggroed?` false)
    (set `self.TargetActor` Target)
    (set `CharacterMovementComponent.MaxWalkSpeed` (`self.AggroedWalkspeed`) (`self.CharacterMovement`))
    (bind _returnvalue (`KismetSystemLibrary.K2_SetTimer` self "FollowTargetDistance" 1.0 true))
    (set `self.FollowDistancetimer` _returnvalue)
    (if (`self.inAttackrange?`)
      (`self.PerformAttack`)
      (else
        (`|AIMoveTo` self (0.0 0.0 0.0) (`self.TargetActor`) (`self.Attackrange`)
          (:`OnSuccess`
            (`self.PerformAttack`)))))))

(event `onReset`
  (set `self.isrunningback?` true)
  (set `self.CurrentAnimationIndex` 0)
  (`KismetSystemLibrary.K2_ClearAndInvalidateTimerHandle` (`self.FollowDistancetimer`))
  (set `self.TargetActor` null)
  (set `self.wasaggroed?` false)
  (`|AIMoveTo` self (`self.Startinglocation`)
    (:`OnSuccess`
      (set `CharacterMovementComponent.MaxWalkSpeed` (`self.Patrolwalkspeed`) (`self.CharacterMovement`))
      (set `self.ispatroling?` true)
      (`self.Patrol`)
      (set `self.isrunningback?` false))))

(fn `FollowTargetDistance`
  (if (> (`KismetMathLibrary.VSize` (- (`self.Startinglocation`) (`self.K2_GetActorLocation`))) (`self.FollowPlayerRadius`))
    (`self.onReset`)
    (return)
    (else
      (return))))

(fn `getnextanimaionIndex`
  (returns (Index :type Integer))
  (bind _returnvalue (+ (`self.CurrentAnimationIndex`) 1))
  (return (`KismetMathLibrary.SelectInt` 0 _returnvalue (> _returnvalue (`KismetArrayLibrary.Array_LastIndex` (`self.AttackAnimations`))))))

(fn `inAttackrange?`
  (returns (Out :type Boolean))
  (return (<= (`self.GetDistanceTo` (`self.TargetActor`) self) (`self.Attackrange`))))

(fn `UserConstructionScript`
  (`parent.UserConstructionScript`))